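; BP_Spline_Spawner places copies of a configurable mesh along a spline in evenly spaced groups.
; The construction script derives the group count from spline length, group size and the two spacing values.
; Nested loops add instances to InstancedSplineMeshes at local-space spline locations and rotations with unit scale.
; A running offset carries each group past the previous one, while an alternative index-based offset calculation is left disconnected.
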(fn ConstructionScript
  (bind _spline (Variables|Default|GetSpline))
  (Components|StaticMesh|SetStaticMesh (Variables|Default|GetInstanced%20Spline%20Meshes) (Variables|Default|GetMesh))
  ;[1 1 1] Calculate Number of groups
  (bind _output_get (LocalVariables|SetNumSplineGroups (Math|Float|Floor (/ (Spline|GetSplineLength (Variables|Default|GetSpline)) (+ (Variables|Default|GetGroup%20Spacing) (* (Variables|Default|GetIndividual%20Spacing) (Variables|Default|GetGroup%20Size)))))))
  (for _index (range 0 (- _output_get 1))
    (for _index_2 (range 1 (Variables|Default|GetGroup%20Size))
      (LocalVariables|SetCurrentOffset (+ (LocalVariables|GetGroupOffsetValue) (* (Variables|Default|GetIndividual%20Spacing) _index_2)))
      (Components|InstancedStaticMesh|AddInstance (Variables|Default|GetInstanced%20Spline%20Meshes) (Math|Transform|MakeTransform (Spline|GetLocationatDistanceAlongSpline _spline (LocalVariables|GetCurrentOffset) "Local") (Spline|GetRotationatDistanceAlongSpline _spline (LocalVariables|GetCurrentOffset) "Local")) false))
    (LocalVariables|SetGroupOffsetValue (+ (LocalVariables|GetCurrentOffset) (Variables|Default|GetGroup%20Spacing)))))